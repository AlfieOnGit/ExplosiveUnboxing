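; Player character that selects actors by looking at them and records the player's confirm or reject response.
; Select line-traces from the camera for WorldDynamic actors implementing the selection interface, deselecting the previous one before selecting an unselected hit.
; Selection raises a response-needed flag, which lets the Confirm and Reject keys record a choice.
; Host-tagged actors mark the response as already received, avoiding a wait for those keys.
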(event EventBeginPlay)

(event Collision|EventActorBeginOverlap
  (params (OtherActor :type Actor%20Object%20Reference)))

(event EventTick
  (params (DeltaSeconds :type Float%20%28single-precision%29)))

(event Input|ActionEvents|InputActionSelect
  (params (Key :type Key%20Structure :default "None"))
  (bind _returnvalue (Game|GetPlayerCameraManager 0))
  (bind _returnvalue_2 (Camera|GetCameraLocation _returnvalue))
  (:Pressed
    (bind (_outhit _returnvalue_3) (Collision|LineTraceForObjects _returnvalue_2 (+ _returnvalue_2 (* (Transformation|GetActorForwardVector _returnvalue) "5000.000000,5000.000000,5000.000000")) (Utilities|Array|MakeArray "ObjectTypeQuery2") false 0 "ForDuration"))
    (if _returnvalue_3
      (if (Utilities|DoesObjectImplementInterface (.hitactor _outhit) "/Game/Blueprints/Select_Actors_Test_Interface.Select_Actors_Test_Interface_C")
        (bind _isselected_ (Class|SelectActorsTestInterface|IsSelected?(Message) (.hitactor _outhit)))
        (if (not _isselected_)
          (Utilities|IsValid (Variables|Default|GetSelected)
            (:Is%20Valid
              (Class|SelectActorsTestInterface|DeselectMyActor(Message) (Variables|Default|GetSelected)))
            (:Is%20Not%20Valid
              _))
          (Class|SelectActorsTestInterface|SelectMyActor(Message) (.hitactor _outhit))
          (Variables|Default|SetSelected (.hitactor _outhit))
          (if (Actor|ActorHasTag (.hitactor _outhit) "Host") ; If Host, will set both as true so doesn't wait for \nconfirm deny keys from other method
            (Variables|Default|SetresponseRecieved true)
            (Variables|Default|SetresponseNeeded true)
            (else
              (Variables|Default|SetresponseRecieved false)
              (Variables|Default|SetresponseNeeded true))))))))

(event Input|ActionEvents|InputActionConfirmKey
  (params (Key :type Key%20Structure :default "None"))
  (:Pressed
    (if (Variables|Default|GetresponseNeeded)
      (Variables|Default|SetconfirmSelection true)
      (Variables|Default|SetresponseRecieved true))))

(event Input|ActionEvents|InputActionRejectKey
  (params (Key :type Key%20Structure :default "None"))
  (:Pressed
    (if (Variables|Default|GetresponseNeeded)
      (Variables|Default|SetconfirmSelection false)
      (Variables|Default|SetresponseRecieved true))))

(fn ConstructionScript)